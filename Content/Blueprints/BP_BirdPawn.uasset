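; BP_BirdPawn is the player bird of a Flappy Bird-style game, hand-animated on Tick without physics.
; Jump starts a decaying rise that tilts the nose up, then gives way to accelerating fall and nose-down rotation.
; While alive but not yet updating, it bobs on a sine wave.
; Body overlaps use component tag counts: untagged contact triggers game over, and end overlap with at most one tag adds score.
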(event OnComponentEndOverlap(Body)
  (params (OverlappedComponent :type Primitive%20Component%20Object%20Reference) (OtherActor :type Actor%20Object%20Reference) (OtherComp :type Primitive%20Component%20Object%20Reference) (OtherBodyIndex :type Integer))
  ;[1 1 1] スコア加算判定
  (if (<= (Utilities|Array|Length (Variables|/Script/Engine.ActorComponent|GetComponentTags OtherComp)) 1)
    (Default|CallAddScoreEvent)))

(event OnComponentBeginOverlap(Body)
  (params (OverlappedComponent :type Primitive%20Component%20Object%20Reference) (OtherActor :type Actor%20Object%20Reference) (OtherComp :type Primitive%20Component%20Object%20Reference) (OtherBodyIndex :type Integer) (bFromSweep :type Boolean) (SweepResult :type Hit%20Result%20Structure%20%28by%20ref%29))
  ;[1 1 1] ゲームオーバー判定
  (if (== (Utilities|Array|Length (Variables|/Script/Engine.ActorComponent|GetComponentTags OtherComp)) 0)
    (Variables|Default|SetIsAlive false)
    (Variables|Default|SetIsUpdate false)
    (Default|CallGameOverEvent)))

(event EventBeginPlay)

(event Collision|EventActorBeginOverlap
  (params (OtherActor :type Actor%20Object%20Reference)))

(event EventTick
  (params (DeltaSeconds :type Float%20%28single-precision%29))
  (bind _returnvalue (Transformation|GetActorLocation))
  (bind _returnvalue_2 (Transformation|GetActorRotation))
  (bind _returnvalue_3 (Transformation|GetActorRotation))
  (bind _returnvalue_4 (Transformation|GetActorLocation))
  (bind _returnvalue_5 (Transformation|GetActorRotation))
  (bind _returnvalue_6 (Transformation|GetActorLocation))
  (bind (_x _y _z) (Math|Vector|BreakVector _returnvalue))
  (bind (_x_2 _y_2 _z_2) (Math|Vector|BreakVector _returnvalue_6))
  (bind (_roll _pitch _yaw) (Math|Rotator|BreakRotator _returnvalue_2))
  (bind (_roll_2 _pitch_2 _yaw_2) (Math|Rotator|BreakRotator _returnvalue_3))
  (bind (_x_3 _y_3) (Math|Vector|BreakVector _returnvalue_4))
  (bind (_roll_3 _pitch_3 _yaw_3) (Math|Rotator|BreakRotator _returnvalue_5))
  (bind _returnvalue_7 (+ _pitch_2 16.0))
  (bind _returnvalue_8 (+ _pitch -2.0))
  (if (Variables|Default|GetIsUpdate)
    (if (Variables|Default|GetIsJump)
      ;[1 1 1] ジャンプ挙動
      (Transformation|SetActorLocation (Math|Vector|MakeVector _x _y (+ _z (Variables|Default|GetJumpPower))) false false)
      (bind _output_get (Variables|Default|SetJumpPower (- (Variables|Default|GetJumpPower) 0.5)))
      (if (<= _output_get 0.0)
        (Variables|Default|SetIsJump false)
        ;[1 1 1] 移動関連処理
        ;;[1 1 1] 落下加速
        (bind _output_get_2 (Variables|Default|SetFallVelocity (+ (Variables|Default|GetFallVelocity) -0.05) :!label _label))
        (Transformation|SetActorLocation (Math|Vector|MakeVector _x_2 _y_2 (+ _z_2 _output_get_2)) false false)
        (if (not (< _returnvalue_8 -65.0))
          (Transformation|SetActorRotation (Math|Rotator|MakeRotator _roll _returnvalue_8 _yaw)))
        (elif (< _returnvalue_7 5e+01)
          (Transformation|SetActorRotation (Math|Rotator|MakeRotator _roll_2 _returnvalue_7 _yaw_2))))
      (else
        (goto _label)))
    (elif (Variables|Default|GetIsAlive)
      ;[1 1 1] 起動前のプレイヤーのゆらぎ
      (if (< (+ (Variables|Default|GetTickCount) 0.01) (Math|Trig|GetPI))
        (Variables|Default|SetTickCount (+ (Variables|Default|GetTickCount) 0.01))
        (else
          (Variables|Default|SetTickCount 0.0)))
      (Transformation|SetActorRotation (Math|Rotator|MakeRotator _roll_3 (Math|Trig|Sin(Radians) 0.0) _yaw_3))
      (Transformation|SetActorLocation (Math|Vector|MakeVector _x_3 _y_3 (* (Math|Trig|Sin(Radians) (Variables|Default|GetTickCount)) 5e+01)) false false))))

(fn ConstructionScript)

(fn Jump
  (if (not (Variables|Default|GetIsJump))
    (Variables|Default|SetIsJump true)
    (Variables|Default|SetJumpPower (Variables|Default|GetJUMP_POWER))
    (Variables|Default|SetFallVelocity (Variables|Default|GetFALL_VELOCITY))))