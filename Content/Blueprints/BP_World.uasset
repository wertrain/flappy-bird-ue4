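; World actor for a side-scrolling pipe obstacle game, likely Flappy Bird style, that builds the level and scrolls the pipes.
; BeginPlay spawns a queue of evenly spaced BP_Pipe actors at random heights and adds static mesh components for floor and background.
; While IsScroll is set, Tick shifts pipes along +X by a fixed per-frame step.
; Pipes past the limit are destroyed, and a new batch spawns when the queue drops below half.
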(event EventBeginPlay
  (CallFunction|CreatePipes (Variables|Default|GetPIPE_INIT_OFFSET))
  (CallFunction|CreateFloor)
  (CallFunction|CreateBackground))

(event Collision|EventActorBeginOverlap
  (params (OtherActor :type Actor%20Object%20Reference)))

(event EventTick
  (params (DeltaSeconds :type Float%20%28single-precision%29))
  (if (Variables|Default|GetIsScroll)
    (CallFunction|MovePipes)))

(fn ConstructionScript)

(fn CreatePipes
  (params (OffsetPos :type Float%20%28single-precision%29))
  (for _index (range 0 (Variables|Default|GetPIPE_MAX_NUM))
    (bind _returnvalue (Game|SpawnActorfromClass "/Game/Blueprints/BP_Pipe.BP_Pipe_C" (Math|Transform|MakeTransform (Math|Vector|MakeVector (- (* (Utilities|Array|Length (Variables|Default|GetPipeQueue)) (Variables|Default|GetPipeInterval)) OffsetPos) 0.0 (Math|Random|RandomFloatinRange -2e+02 2e+02))) "Undefined" 0 0))
    (bind _output_get (LocalVariables|SetTempPipe _returnvalue))
    (Utilities|Array|Add (Variables|Default|GetPipeQueue) _output_get)
    (Rendering|SetVisibility (Variables|/Script/Engine.Actor|GetRootComponent _output_get) true false)))

(fn MovePipes
  ;[1 1 1] パイプの移動処理
  (for _array_element (Variables|Default|GetPipeQueue)
    (LocalVariables|SetTempPipe _array_element)
    (if (> (.X (Math|Vector|BreakVector (Transformation|GetActorLocation (LocalVariables|GetTempPipe)))) 7.5e+02)
      ;[1 1 1] 位置が一定の座標になればパイプを削除
      (Actor|DestroyActor (LocalVariables|GetTempPipe))
      (Utilities|Array|RemoveItem (Variables|Default|GetPipeQueue) (LocalVariables|GetTempPipe))
      (if (< (Utilities|Array|Length (Variables|Default|GetPipeQueue)) (/ (Variables|Default|GetPIPE_MAX_NUM) 2))
        (CallFunction|CreatePipes (* (Variables|Default|GetPIPE_INIT_OFFSET) -0.5)))
      (else
        (Transformation|SetActorLocation (LocalVariables|GetTempPipe) (Math|Vector|MakeVector (+ (.X (Math|Vector|BreakVector (Transformation|GetActorLocation (LocalVariables|GetTempPipe)))) (Variables|Default|GetPipeSpeed)) (.Y (Math|Vector|BreakVector (Transformation|GetActorLocation (LocalVariables|GetTempPipe)))) (.Z (Math|Vector|BreakVector (Transformation|GetActorLocation (LocalVariables|GetTempPipe))))) false true)))))

(fn CreateFloor
  (for _index (range 0 (Variables|Default|GetFLOOR_MAX_NUM))
    (AddComponent|AddStaticMeshComponent false (Math|Transform|MakeTransform (Math|Vector|MakeVector (+ (* _index 1e+02) -1.5e+03) 0.0 -3e+02)))))

(fn CreateBackground
  (AddComponent|AddStaticMeshComponent false (Math|Transform|MakeTransform "0,563.173096,460.764740" "0, 0,90.000000" "20.000000,20.000000,20.000000")))